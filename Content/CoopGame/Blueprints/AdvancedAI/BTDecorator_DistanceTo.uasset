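; Behavior tree decorator that passes when the controlled pawn is within a maximum distance of a target actor.
; It reads the target from a blackboard key, casts it to an Actor and compares the straight-line distance between the two locations against MaxDistanceTo.
; The check fails when the key holds no valid actor.
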(fn PerformConditionCheckAI
  (params (OwnerController :type AI%20Controller%20Object%20Reference) (ControlledPawn :type Pawn%20Object%20Reference))
  (bind _asactor (Utilities|Casting|CastToActor (Class|BTFunctionLibrary|GetBlackboardValueasObject (Variables|Default|GetTargetActorKey)))
    (:then
      (return (< (Math|Vector|VectorLength (- (Transformation|GetActorLocation ControlledPawn) (Transformation|GetActorLocation _asactor))) (Variables|Default|GetMaxDistanceTo))))
    (:CastFailed
      (return false))))