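; BP_GameMode is the game mode Blueprint that spawns enemy or AI bots at locations chosen by the Environment Query System.
; SpawnBot runs the EQS_FindSpawnLocation query in random-best-25% mode and prints a debug "Hello".
; On query success, it spawns either BP_AICharacter or BP_TrackerBot, weighted by AdvancedAIRate, at a random result location.
; Spawning adjusts around collisions and is skipped if still blocked.
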(event Custom|OnQueryFinishedEvent_Event_0
  (params (QueryInstance :type Env%20Query%20Instance%20Blueprint%20Wrapper%20Object%20Reference) (QueryStatus :type EEnvQueryStatus%20Enum :default "Processing"))
  (switch Utilities|FlowControl|Switch|SwitchonEEnvQueryStatus QueryStatus
    (:Success
      (bind _resultlocations (AI|EQS|GetQueryResultsasLocations QueryInstance))
      (Game|SpawnActorfromClass (select (< (Math|Random|RandomFloatinRange 0.0 1.0) (Variables|Default|GetAdvancedAIRate)) "/Game/CoopGame/Blueprints/AdvancedAI/BP_AICharacter.BP_AICharacter_C" "/Game/CoopGame/Blueprints/AI/BP_TrackerBot.BP_TrackerBot_C") (Math|Transform|MakeTransform (.OutItem (Utilities|Array|Random _resultlocations)) "0, 0, 0" "1,1,1") "AdjustIfPossibleButDontSpawnIfColliding" 0))))

(event EventSpawnBot
  (bind _returnvalue (AI|EQS|RunEQSQuery "/Game/CoopGame/Blueprints/AI/EQS/EQS_FindSpawnLocation.EQS_FindSpawnLocation" self "RandomBest25Pct"))
  (EventDispatchers|AssignOnQueryFinishedEvent _returnvalue (delegate Custom|OnQueryFinishedEvent_Event_0))
  (Development|PrintString "Hello"))

(fn ConstructionScript)